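; BarrierBP is a barrier of three boards that can be built up and torn down one board at a time.
; BuildBarrier reveals the next board and enables its collision, using the BoardsVisible count to pick the component, up to three.
; DestroyBarrier reverses this for the most recent board, stopping at zero.
; Each successful build also starts a ten-second delay, then repeatedly calls DestroyBarrier, clearing all visible boards.
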(event Custom|BuildBarrier
  (bind _boardsvisible (Variables|Default|GetBoardsVisible))
  (bind _returnvalue (- _boardsvisible 1))
  (if (not (== (Variables|Default|GetBoardsVisible) 3))
    (Math|Integer|IncrementInt _boardsvisible
      (:%20%20
        (Rendering|SetVisibility (Utilities|Select :Index _returnvalue :Option%200 (Variables|Default|GetBoard1) :Option%201 (Variables|Default|GetBoard2) :Option%202 (Variables|Default|GetBoard3)) true false)
        (Collision|SetCollisionEnabled (Utilities|Select :Index _returnvalue :Option%200 (Variables|Default|GetBoard1) :Option%201 (Variables|Default|GetBoard2) :Option%202 (Variables|Default|GetBoard3)) "QueryAndPhysics")
        (Utilities|FlowControl|Delay 1e+01)
        (for _index (range 0 7)
          (CallFunction|DestroyBarrier))))))

(event Custom|DestroyBarrier
  (bind _boardsvisible (Variables|Default|GetBoardsVisible))
  (bind _boardsvisible_2 (Variables|Default|GetBoardsVisible))
  (if (not (== _boardsvisible 0))
    (Math|Integer|DecrementInt _boardsvisible
      (:%20%20
        (Rendering|SetVisibility (Utilities|Select :Index _boardsvisible_2 :Option%200 (Variables|Default|GetBoard1) :Option%201 (Variables|Default|GetBoard2) :Option%202 (Variables|Default|GetBoard3)) false false)
        (Collision|SetCollisionEnabled (Utilities|Select :Index _boardsvisible_2 :Option%200 (Variables|Default|GetBoard1) :Option%201 (Variables|Default|GetBoard2) :Option%202 (Variables|Default|GetBoard3)) "NoCollision")))))

(event EventBeginPlay)

(event Collision|EventActorBeginOverlap
  (params (OtherActor :type Actor%20Object%20Reference)))

(event EventTick
  (params (DeltaSeconds :type Float%20%28single-precision%29)))

(fn ConstructionScript)