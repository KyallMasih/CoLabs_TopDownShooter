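; Door Blueprint that swings open once the player has collected enough keycards.
; CollectKeycard increments a counter, and Interactfordooropening compares it to the required maximum before triggering the opening through a DoOnce, so it fires only once.
; Opendoor plays a Timeline that lerps the Door's relative yaw to swing it open, with no closing logic.
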(event Custom|Open%20door
  ;[1 1 1] Opening of the door of the rotation by 120 (depending on the mesh)
  (bind _door_open (Timeline|Timeline Play)
    (:Update
      (Transformation|SetRelativeRotation (Variables|Default|GetDoor) (Math|Rotator|MakeRotator 0.0 0.0 (Math|Float|Lerp 0.0 1.2e+02 _door_open)) false false))))

(event Custom|Collect%20Keycard
  ;[1 1 1] Collecting the keycards no more no less to open the door
  (Math|Integer|IncrementInt (Variables|Default|GetCurrenItemsCollected)))

(event Custom|Interact%20for%20door%20opening
  (if (>= (Variables|Default|GetCurrenItemsCollected) (Variables|Default|GetMaxItemsCollected))
    (Utilities|FlowControl|DoOnce false
      (:Completed
        (CallFunction|OpenDoor)))))

(event EventBeginPlay)

(event Collision|EventActorBeginOverlap
  (params (OtherActor :type Actor%20Object%20Reference)))

(event EventTick
  (params (DeltaSeconds :type Float%20%28single-precision%29)))

(fn ConstructionScript)