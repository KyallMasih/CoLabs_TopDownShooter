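; BP_door is a swinging door that opens and closes on interaction once three keycard flags are set.
; Its PickUpKeycard event sets all three flags at once, and Interact does nothing unless all are true.
; A FlipFlop alternately plays and reverses a timeline that lerps the static mesh's relative yaw between closed and open angles.
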(event EventBeginPlay)

(event Collision|EventActorBeginOverlap
  (params (OtherActor :type Actor%20Object%20Reference)))

(event EventTick
  (params (DeltaSeconds :type Float%20%28single-precision%29)))

(event EventPickUpKeycard
  (Utilities|FlowControl|Sequence
    (:then_1
      (Variables|Default|SetHas%20Keycard1? true))
    (:then_2
      (Variables|Default|SetHas%20Keycard2? true))
    (:then_3
      (Variables|Default|SetHas%20Keycard3? true))))

(event EventInteract
  (if (Variables|Default|GetHas%20Keycard1?)
    (if (Variables|Default|GetHas%20Keycard2?)
      (if (Variables|Default|GetHas%20Keycard3?)
        (Utilities|FlowControl|FlipFlop
          (:A
            (bind _door_track (Timeline|Door%20timeline Play)
              (:Update
                (Transformation|SetRelativeRotation (Variables|Default|GetStaticMesh) (Math|Rotator|MakeRotator 0.0 0.0 (Math|Float|Lerp 0.0 1.1e+02 _door_track)) false false))))
          (:B
            (Timeline|Door%20timeline Reverse)))))))

(fn ConstructionScript)