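; BP_Projectile is a bullet actor that damages enemies and awards score to the top-down player character.
; Its collision sphere's begin-overlap event casts the hit actor to BP_TurrentEnemy and BP_Enemy in sequence.
; BP_Enemy loses health and is destroyed at zero, incrementing the player's Score.
; The turret branch writes Health back unchanged and, if already depleted, increments Score and sets Points without destroying the turret.
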(event OnComponentBeginOverlap(Sphere_Collision)
  (params (OverlappedComponent :type Primitive%20Component%20Object%20Reference) (OtherActor :type Actor%20Object%20Reference) (OtherComp :type Primitive%20Component%20Object%20Reference) (OtherBodyIndex :type Integer) (bFromSweep :type Boolean) (SweepResult :type Hit%20Result%20Structure%20%28by%20ref%29))
  ;[1 1 1] Bullet Damage
  (Utilities|FlowControl|Sequence
    (:then_0
      (bind _asbp_turrent_enemy (Utilities|Casting|CastToBP_TurrentEnemy OtherActor))
      (Variables|/Game/DevSpaces/Fahim/Blueprints/BP_TurrentEnemy.BP_TurrentEnemy_C|SetHealth _asbp_turrent_enemy (Variables|/Game/DevSpaces/Fahim/Blueprints/BP_TurrentEnemy.BP_TurrentEnemy_C|GetHealth _asbp_turrent_enemy))
      (if (<= (Variables|/Game/DevSpaces/Fahim/Blueprints/BP_TurrentEnemy.BP_TurrentEnemy_C|GetHealth _asbp_turrent_enemy) 0.0)
        (bind _asbp_top_down_character (Utilities|Casting|CastToBP_TopDownCharacter (Game|GetPlayerCharacter 0)))
        (Math|Integer|IncrementInt (Variables|/Game/TopDown/Blueprints/BP_TopDownCharacter.BP_TopDownCharacter_C|GetScore _asbp_top_down_character)
          (:%20%20
            (Variables|Default|SetPoints 2)))))
    (:then_1
      (bind _asbp_enemy (Utilities|Casting|CastToBP_Enemy OtherActor))
      (Variables|/Game/DevSpaces/Kyall/EnemyAI/BP_Enemy.BP_Enemy_C|SetHealth _asbp_enemy (- (Variables|/Game/DevSpaces/Kyall/EnemyAI/BP_Enemy.BP_Enemy_C|GetHealth _asbp_enemy) 5e+01))
      (if (<= (Variables|/Game/DevSpaces/Kyall/EnemyAI/BP_Enemy.BP_Enemy_C|GetHealth _asbp_enemy) 0.0)
        (Utilities|FlowControl|Sequence
          (:then_0
            (bind _asbp_top_down_character_2 (Utilities|Casting|CastToBP_TopDownCharacter (Game|GetPlayerCharacter 0)))
            (Math|Integer|IncrementInt (Variables|/Game/TopDown/Blueprints/BP_TopDownCharacter.BP_TopDownCharacter_C|GetScore _asbp_top_down_character_2)))
          (:then_1
            (Actor|DestroyActor _asbp_enemy)))))))

(event EventBeginPlay)

(event Collision|EventActorBeginOverlap
  (params (OtherActor :type Actor%20Object%20Reference)))

(event EventTick
  (params (DeltaSeconds :type Float%20%28single-precision%29)))

(fn ConstructionScript)