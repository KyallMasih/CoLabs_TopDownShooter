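; BP_boss is a stationary boss that turns to face the player, fires projectiles and shows a health bar widget.
; Tick interpolates its rotation toward the player, while Shoot re-arms its own looping timer to spawn a BP_BossProjectile from Arrow1.
; BP_Projectile overlaps on Box destroy the projectile, reduce Health and update the bar.
; At zero Health the boss destroys itself and displays the win screen.
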(event OnComponentBeginOverlap(Box)
  (params (OverlappedComponent :type Primitive%20Component%20Object%20Reference) (OtherActor :type Actor%20Object%20Reference) (OtherComp :type Primitive%20Component%20Object%20Reference) (OtherBodyIndex :type Integer) (bFromSweep :type Boolean) (SweepResult :type Hit%20Result%20Structure%20%28by%20ref%29))
  ;[1 1 1] Destroying Projectile
  (bind _asbp_projectile (Utilities|Casting|CastToBP_Projectile OtherActor))
  (Actor|DestroyActor _asbp_projectile)
  (bind _output_get (Variables|Default|SetHealth (- (Variables|Default|GetHealth) 2e+01)))
  (Development|PrintString (Utilities|String|ToString(Float) _output_get))
  (Variables|/Game/DevSpaces/Lucas/WB_BossHealthBar.WB_BossHealthBar_C|SetHealth (Variables|Default|GetBossHealthBar) (Variables|Default|GetHealth))
  (if (<= (Variables|Default|GetHealth) 0.0)
    (Actor|DestroyActor)
    (bind _returnvalue (UserInterface|CreateWidget "/Game/TopDown/Blueprints/UI/BP_WinScreen.BP_WinScreen_C"))
    (UserInterface|Viewport|AddtoViewport _returnvalue 0)))

(event Custom|Shoot
  (Utilities|Time|SetTimerbyEvent (delegate Custom|Shoot) 1.0 true)
  (Game|SpawnActorfromClass "/Game/DevSpaces/Lucas/BP_BossProjectile.BP_BossProjectile_C" (Transformation|GetWorldTransform (Variables|Default|GetArrow1)) "Undefined" "MultiplyWithRoot" 0 0))

(event EventTick
  (params (DeltaSeconds :type Float%20%28single-precision%29))
  ;[1 1 1] AI Movement
  (Transformation|SetActorRotation (Math|Interpolation|RInterpTo (Transformation|GetActorRotation) (Math|Rotator|FindLookatRotation (Transformation|GetActorLocation) (Transformation|GetActorLocation (Game|GetPlayerCharacter 0))) DeltaSeconds 0.0)))

(event EventBeginPlay
  (CallFunction|Shoot)
  (bind _returnvalue (UserInterface|CreateWidget "/Game/DevSpaces/Lucas/WB_BossHealthBar.WB_BossHealthBar_C"))
  (bind _output_get (Variables|Default|SetBossHealthBar _returnvalue))
  (UserInterface|Viewport|AddtoViewport _output_get 0)
  (Variables|/Game/DevSpaces/Lucas/WB_BossHealthBar.WB_BossHealthBar_C|SetMaxHealth _output_get (Variables|Default|GetHealth)))

(fn ConstructionScript)