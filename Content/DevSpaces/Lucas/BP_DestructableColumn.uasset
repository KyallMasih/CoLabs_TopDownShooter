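; A destructible column that takes damage from boss projectiles.
; When a BP_BossProjectile overlaps its Box, the projectile is destroyed and column health drops by a fixed amount.
; At zero health, the Cube mesh swaps to a destroyed column model, resets scale and shifts downward, and the Box is removed so it stops blocking further projectiles.
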(event OnComponentBeginOverlap(Box)
  (params (OverlappedComponent :type Primitive%20Component%20Object%20Reference) (OtherActor :type Actor%20Object%20Reference) (OtherComp :type Primitive%20Component%20Object%20Reference) (OtherBodyIndex :type Integer) (bFromSweep :type Boolean) (SweepResult :type Hit%20Result%20Structure%20%28by%20ref%29))
  (bind _cube (Variables|Default|GetCube))
  (bind _asbp_boss_projectile (Utilities|Casting|CastToBP_BossProjectile OtherActor))
  (Actor|DestroyActor _asbp_boss_projectile)
  (Variables|Default|SetColumnHealth (- (Variables|Default|GetColumnHealth) 15.0))
  (if (<= (Variables|Default|GetColumnHealth) 0.0)
    (Variables|Default|SetWorldLoc (Transformation|GetWorldLocation _cube))
    (Components|StaticMesh|SetStaticMesh _cube "/Game/DevSpaces/Lucas/ColumnDest_9F1924CF.ColumnDest_9F1924CF")
    (Transformation|SetWorldScale3D _cube "1.000000,1.000000,1.000000")
    (Transformation|SetWorldLocation _cube (- (Variables|Default|GetWorldLoc) "0.000000,0.000000,60.000000") false false)
    (Components|DestroyComponent (Variables|Default|GetBox))))

(event Collision|EventActorBeginOverlap
  (params (OtherActor :type Actor%20Object%20Reference)))

(fn ConstructionScript)