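; BP_Tower1 is a tower actor that reacts to enemies reaching it and shows its health on a widget.
; When a BP_TowerEnemy overlaps its Box component, the tower adds a fixed amount to Health, rather than subtracting it, and destroys the enemy.
; UpdateHealthBar copies Health into the WB_TowerHealthBar inside the HealthBar widget component, on BeginPlay and after each such overlap.
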(event OnComponentBeginOverlap(Box)
  (params (OverlappedComponent :type Primitive%20Component%20Object%20Reference) (OtherActor :type Actor%20Object%20Reference) (OtherComp :type Primitive%20Component%20Object%20Reference) (OtherBodyIndex :type Integer) (bFromSweep :type Boolean) (SweepResult :type Hit%20Result%20Structure%20%28by%20ref%29))
  (bind _asbp_tower_enemy (Utilities|Casting|CastToBP_TowerEnemy OtherActor))
  (Utilities|IsValid _asbp_tower_enemy
    (:Is%20Valid
      (Variables|Default|SetHealth (+ (Variables|Default|GetHealth) 1e+01))
      (CallFunction|UpdateHealthBar)
      (Actor|DestroyActor _asbp_tower_enemy))))

(event EventBeginPlay
  (CallFunction|UpdateHealthBar))

(event Collision|EventActorBeginOverlap
  (params (OtherActor :type Actor%20Object%20Reference)))

(event EventTick
  (params (DeltaSeconds :type Float%20%28single-precision%29)))

(fn ConstructionScript)

(fn UpdateHealthBar
  (bind _aswb_tower_health_bar (Utilities|Casting|CastToWB_TowerHealthBar (UserInterface|GetUserWidgetObject (Variables|Default|GetHealthBar))))
  (Utilities|IsValid _aswb_tower_health_bar
    (:Is%20Valid
      (Variables|/Game/DevSpaces/Kameron/Bps/WB_TowerHealthBar.WB_TowerHealthBar_C|SetHealth _aswb_tower_health_bar (Variables|Default|GetHealth))
      (return))))